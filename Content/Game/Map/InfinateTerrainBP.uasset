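; InfinateTerrainBP is a self-spawning terrain segment for an endless side-scroller.
; On BeginPlay it spawns one random obstacle, a cactus or eagle variant, at its Obstacles point, then destroys itself after a fixed delay.
; When the SideScrollerCharacter overlaps its Box trigger, it spawns another copy of itself at SpawnLocation, chaining segments endlessly.
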(event OnComponentBeginOverlap(Box)
  (params (OverlappedComponent :type Primitive%20Component%20Object%20Reference) (OtherActor :type Actor%20Object%20Reference) (OtherComp :type Primitive%20Component%20Object%20Reference) (OtherBodyIndex :type Integer) (bFromSweep :type Boolean) (SweepResult :type Hit%20Result%20Structure%20%28by%20ref%29))
  ;[1 1 1] Spawn Terrain
  (Utilities|Casting|CastToSideScrollerCharacter OtherActor)
  (Game|SpawnActorfromClass "InfinateTerrainBP_C" (Transformation|GetWorldTransform (Variables|Default|GetSpawnLocation)) "Undefined" 0 0))

(event EventBeginPlay
  (bind _obstacles (Variables|Default|GetObstacles))
  (bind _returnvalue (Transformation|GetWorldTransform _obstacles))
  (Utilities|FlowControl|Sequence
    (:then_0
      (switch int (Math|Random|RandomIntegerinRange 0 4)
        (:0
          (Game|SpawnActorfromClass "/Game/Game/Obstacles/CactusBP.CactusBP_C" _returnvalue "Undefined" 0 0))
        (:1
          (Game|SpawnActorfromClass "/Game/Game/Obstacles/Cactus2BP.Cactus2BP_C" _returnvalue "Undefined" 0 0))
        (:2
          (Game|SpawnActorfromClass "/Game/Game/Obstacles/Cactus3BP.Cactus3BP_C" _returnvalue "Undefined" 0 0))
        (:3
          (Game|SpawnActorfromClass "/Game/Game/Obstacles/EagleBP.EagleBP_C" _returnvalue "Undefined" 0 0))
        (:4
          (Game|SpawnActorfromClass "/Game/Game/Obstacles/EagleBP_2.EagleBP_2_C" _returnvalue "Undefined" 0 0))))
    (:then_1
      (Utilities|FlowControl|Delay 1e+01)
      (Actor|DestroyActor))))

(fn ConstructionScript)